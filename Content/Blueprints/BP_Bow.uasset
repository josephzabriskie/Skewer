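; Player bow that aims, charges and fires skewer projectiles, scoring points when they stab a wall.
; Desktop aiming traces under the mouse, while touch aims inversely, slingshot-style.
; Holding fire runs a looping timer that builds power, draws back the arrow and debug-draws the predicted path; a Gate resumes charging after cooldown if still held.
; Release launches a skewer by impulse and binds its wall-stab event to update the HUD score.
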(event Custom|FireSkewer
  (params (Velocity :type Vector))
  (bind _arrowmesh (Variables|Default|GetArrowMesh))
  (bind _returnvalue (Transformation|GetWorldTransform _arrowmesh))
  ;[1 1 1] Spawn and launch a skewer
  (bind _returnvalue_2 (Game|SpawnActorfromClass "/Game/Blueprints/SkewerProjectile.SkewerProjectile_C" (Math|Transform|MakeTransform (.location _returnvalue) (.rotation _returnvalue) (.scale _returnvalue)) "Undefined" 0 0))
  (Physics|AddImpulse (Variables|/Game/Blueprints/SkewerProjectile.SkewerProjectile_C|GetSkewerMesh _returnvalue_2) Velocity "None" false)
  (CallFunction|AddandBindSkewer _returnvalue_2))

(event Custom|TimedChargeIncrease
  (bind _firepowerminmax (Variables|Default|GetFirePowerMinMax))
  (bind _arrowmesh (Variables|Default|GetArrowMesh))
  (bind _firepowerminmax_2 (Variables|Default|GetFirePowerMinMax))
  (bind _bow (Variables|Default|GetBow))
  (bind _relativelocation (Variables|/Script/Engine.SceneComponent|GetRelativeLocation _arrowmesh))
  ;[1 1 1] Incremental increase of bow charge
  (Variables|Default|SetCurrentFireVeloctiy (Math|Float|Clamp(Float) (+ (Variables|Default|GetCurrentFireVeloctiy) (* (Variables|Default|GetChargeRate) (Variables|Default|GetChargingUpdateInterval))) (.x _firepowerminmax) (.y _firepowerminmax)))
  (bind _output_get (Variables|Default|SetLaunchVelocity (* (Math|Vector|GetForwardVector (Transformation|GetWorldRotation _bow)) (Variables|Default|GetCurrentFireVeloctiy))))
  (Class|GameplayStatics|BlueprintPredictProjectilePathbyTraceChannel (Transformation|GetWorldLocation _bow) _output_get false 1e+01 "ECC_WorldStatic" false (Utilities|Array|MakeArray self) "ForDuration" (Variables|Default|GetChargingUpdateInterval) 15.0 1.0)
  (Transformation|SetRelativeLocation (Variables|Default|GetArrowMesh) (Math|Vector|MakeVector (* (/ (- (Variables|Default|GetCurrentFireVeloctiy) (.x _firepowerminmax_2)) (- (.y _firepowerminmax_2) (.x _firepowerminmax_2))) (Variables|Default|GetArrowDrawDistance)) (.y _relativelocation) (.z _relativelocation)) false false) ; Draw back arrow based on fire velocity
)

(event Custom|ResetShot
  ;[1 1 1] Let player fire an arrow again!
  (Rendering|SetVisibility (Variables|Default|GetArrowMesh) true false)
  (Variables|Default|SetbFireOnCooldown false)
  (CallFunction|StartCharge) ; Start charge again, gate will be open if button is pressed, otherwise this will fizzle
)

(event Custom|StartCharge
  ;[1 1 1] Start charging, gated by InputAction Fire being currently down
  (Utilities|FlowControl|Gate true :!label _label
    (:Exit
      (if (and (not (Variables|Default|GetbFireOnCooldown)) (Variables|Default|GetbFiringEnabled))
        (bind _returnvalue (Utilities|Time|SetTimerbyEvent (delegate Custom|TimedChargeIncrease) (Variables|Default|GetChargingUpdateInterval) true))
        (Variables|Default|SetChargingTimer _returnvalue)
        (Variables|Default|SetbFireOnCooldown true)
        (goto _label Close)))))

(event Custom|EndCharge
  ;[1 1 1] End charging, potentially fire off a new skewer if one's been charging
  (if (Utilities|Time|IsValidTimerHandle (Variables|Default|GetChargingTimer)) ; If charging a shot
    (CallFunction|FireSkewer (Variables|Default|GetLaunchVelocity))
    (Variables|Default|SetCurrentFireVeloctiy (.x (Variables|Default|GetFirePowerMinMax)))
    (Utilities|Time|ClearandInvalidateTimerbyHandle (Variables|Default|GetChargingTimer))
    (Transformation|SetRelativeLocation (Variables|Default|GetArrowMesh) "0, 0, 0" false false)
    (Rendering|SetVisibility (Variables|Default|GetArrowMesh) false false)
    (Utilities|Time|SetTimerbyEvent (delegate Custom|ResetShot) (Variables|Default|GetFireDelay))))

(event EventBeginPlay
  (Utilities|FlowControl|Sequence
    (:then_0
      ;[1 1 1] Set Up Bow
      (Transformation|SetWorldRotation (Variables|Default|GetAimTarget) "0, 0, 0" false false)
      (Variables|Default|SetCurrentFireVeloctiy (.x (Variables|Default|GetFirePowerMinMax))))
    (:then_1
      (bind _returnvalue (UserInterface|CreateWidget "/Game/Widgets/SkewerHUD.SkewerHUD_C"))
      (bind _output_get (Variables|Scoring|SetHUDRef _returnvalue))
      (UserInterface|Viewport|AddtoViewport _output_get 0))))

(event EventTick
  (params (DeltaSeconds :type Float%20%28single-precision%29))
  (bind _returnvalue (Game|GetPlayerController 0))
  (bind (_worldlocation _worlddirection) (Game|Player|ConvertMouseLocationToWorldSpace _returnvalue))
  (Utilities|FlowControl|Sequence
    (:then_0
      ;[1 1 1] Targeting Cursor for PC cursor aiming (bow points at mouse)
      (switch string (Game|GetPlatformName) ; Show cursor only on PC platforms
        (:Windows
          _)
        (:Mac
          _)
        (:Linux
          _))
      (if (not (Variables|Default|GetbCursorAsTouch_DEV_))
        (bind _outhit (Collision|LineTraceByChannel _worldlocation (+ _worldlocation (* _worlddirection 5e+04)) "TraceTypeQuery3" false 0 "None" false "(R=1.000000,G=0.000000,B=0.000000,A=1.000000)" "(R=0.000000,G=1.000000,B=0.000000,A=1.000000)" 5e+01))
        (CallFunction|AimBowatTarget (.Location (Collision|BreakHitResult _outhit)) false)))))

(event Input|ActionEvents|InputActionFire
  (params (Key :type Key%20Structure :default "None"))
  (:Pressed
    (Utilities|FlowControl|Sequence
      (:then_0
        ;[1 1 1] Start charging, gated by InputAction Fire being currently down
        (Utilities|FlowControl|Gate true) ; enters at Open
      )
      (:then_1
        (CallFunction|StartCharge))))
  (:Released
    (CallFunction|EndCharge)
    (Utilities|FlowControl|Gate true) ; enters at Close
  ))

(event Input|TouchEvents|InputTouch
  (params (Location :type Vector) (FingerIndex :type ETouchIndex%20Enum))
  (bind (_x _y) (Math|Vector|BreakVector Location))
  (bind _returnvalue (Game|GetPlayerController 0))
  (bind (_worldlocation _worlddirection) (Class|PlayerController|DeprojectScreenPositiontoWorld _returnvalue _x _y))
  (:Pressed
    (Utilities|FlowControl|Sequence ; Touch Input handles both startCharge and aim
      (:then_0
        ;[1 1 1] Touch Aiming (Inversed)
        (bind _outhit (Collision|LineTraceByChannel _worldlocation (+ _worldlocation (* _worlddirection 5e+04)) "TraceTypeQuery3" false 0 "None" false "(R=1.000000,G=0.000000,B=0.000000,A=1.000000)" "(R=0.000000,G=1.000000,B=0.000000,A=1.000000)" 5e+01 :!label _label))
        (CallFunction|AimBowatTarget (.Location (Collision|BreakHitResult _outhit)) true))
      (:then_1
        (Utilities|FlowControl|Sequence
          (:then_0
            ;[1 1 1] Start charging, gated by InputAction Fire being currently down
            (Utilities|FlowControl|Gate true) ; enters at Open
          )
          (:then_1
            (CallFunction|StartCharge))))))
  (:Released
    (CallFunction|EndCharge)
    (Utilities|FlowControl|Gate true) ; enters at Close
  )
  (:Moved
    (goto _label)))

(fn ConstructionScript)

(fn AimBowatTarget
  (params (NewAimTargetWorldLoc :type Vector) (InverseAim :type Boolean))
  (bind _aimtarget (Variables|Default|GetAimTarget))
  (bind _bow (Variables|Default|GetBow))
  (bind _aimtarget_2 (Variables|Default|GetAimTarget))
  (bind _relativelocation (Variables|/Script/Engine.SceneComponent|GetRelativeLocation _bow))
  (bind _relativelocation_2 (Variables|/Script/Engine.SceneComponent|GetRelativeLocation _aimtarget))
  (Transformation|SetWorldLocation _aimtarget_2 (Math|Vector|MakeVector (.x (Transformation|GetWorldLocation _aimtarget_2)) (.y NewAimTargetWorldLoc) (.z NewAimTargetWorldLoc)) false false)
  (Transformation|SetRelativeRotation (Variables|Default|GetBow) (Math|Rotator|SelectRotator (Math|Rotator|FindLookatRotation _relativelocation_2 _relativelocation) (Math|Rotator|FindLookatRotation _relativelocation _relativelocation_2) InverseAim) false false))

(fn AddtoScore
  (params (AddScore :type Integer))
  (bind _output_get (Variables|Scoring|SetScore (+ AddScore (Variables|Scoring|GetScore))))
  (Default|SetScore (Variables|/Game/Widgets/SkewerHUD.SkewerHUD_C|GetScoreDisplay (Variables|Scoring|GetHUDRef)) _output_get))

(fn AddandBindSkewer
  (params (NewSkewer :type Skewer%20Projectile%20Object%20Reference))
  (Utilities|Array|AddUnique (Variables|Scoring|GetSkewers) NewSkewer)
  (EventDispatchers|BindEventtoWallStabbed NewSkewer (EventDispatchers|CreateEvent :!event ReceiveSkewerWallStabbed)))

(fn RemoveandUnbindSkewer
  (params (RemoveSkewer :type Skewer%20Projectile%20Object%20Reference))
  (Utilities|Array|RemoveItem (Variables|Scoring|GetSkewers) RemoveSkewer)
  (EventDispatchers|UnbindEventfromWallStabbed RemoveSkewer (EventDispatchers|CreateEvent :!event ReceiveSkewerWallStabbed)))

(fn ReceiveSkewerWallStabbed
  (params (Skewer :type Skewer%20Projectile%20Object%20Reference))
  (bind _pointvalue (Default|GetPointValue Skewer))
  (CallFunction|AddtoScore _pointvalue)
  (CallFunction|RemoveandUnbindSkewer Skewer))

(fn SetAllowFiring
  (params (bAllowFiring :type Boolean))
  (bind _output_get (Variables|Default|SetbFiringEnabled bAllowFiring))
  (if (not _output_get)
    (CallFunction|EndCharge) ; This will release a held charge if one's going, do nothing otherwise
  ))