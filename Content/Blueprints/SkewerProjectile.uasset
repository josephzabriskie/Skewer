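; Physics-driven skewer projectile that turns along its flight arc, spearing food actors into a spaced stack and slowing with each catch.
; Surfaces tagged SkewerStab stop it when impact is fast enough, or moderate and head-on by line trace.
; Catches and normal wall sticks rescore the stack from base points, set bonuses and percentage combo multipliers, popping the total on a widget.
; On destruction, it releases or destroys its food.
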(event OnComponentBeginOverlap(PointCollision)
  (params (OverlappedComponent :type Primitive%20Component%20Object%20Reference) (OtherActor :type Actor%20Object%20Reference) (OtherComp :type Primitive%20Component%20Object%20Reference) (OtherBodyIndex :type Integer) (bFromSweep :type Boolean) (SweepResult :type Hit%20Result%20Structure%20%28by%20ref%29))
  (bind (_asbp_food_base _bsuccess) (Utilities|Casting|CastToBP_FoodBase OtherActor))
  (if (Actor|ActorHasTag OtherActor "SkewerStab")
    (CallFunction|CheckWallStab OtherComp)
    (elif _bsuccess
      (CallFunction|TryAttachFood _asbp_food_base))))

(event EventBeginPlay)

(event Collision|EventActorBeginOverlap
  (params (OtherActor :type Actor%20Object%20Reference)))

(event EventTick
  (params (DeltaSeconds :type Float%20%28single-precision%29))
  (if (Variables|Default|GetbDoArcAdjust)
    (CallFunction|SetAnglebyVelocity DeltaSeconds)
    (Transformation|SetWorldRotation (Variables|Default|GetWidget) "0, 0, 0" false false)))

(event EventDestroyed
  (for _array_element (Variables|Default|GetAttachedFoods)
    (bind _asbp_food_base (Utilities|Casting|CastToBP_FoodBase _array_element))
    (if (Variables|Default|GetbReleaseOnDestroy)
      (Default|DetachfromSkewer _asbp_food_base)
      (else
        (Actor|DestroyActor _asbp_food_base)))))

(fn ConstructionScript)

(fn CheckWallStab
  (params (OtherComponent :type Primitive%20Component%20Object%20Reference))
  (bind _skewermesh (Variables|Default|GetSkewerMesh))
  (bind _returnvalue (Transformation|GetWorldLocation _skewermesh))
  (bind _returnvalue_2 (Math|Vector|GetUpVector _skewermesh))
  (bind _returnvalue_3 (Class|PrimitiveComponent|GetPhysicsLinearVelocityatPoint (Variables|Default|GetSkewerMesh) (Transformation|GetWorldLocation (Variables|Default|GetPointCollision)) "None"))
  (if (> (Math|Vector|VectorLength _returnvalue_3) 1.8e+03)
    (Transformation|AddActorWorldOffset (* (Math|Vector|GetUpVector (Variables|Default|GetSkewerMesh)) (Math|Random|RandomFloatinRange 15.0 3e+01)) :!label _label)
    (Physics|SetSimulatePhysics (Variables|Default|GetSkewerMesh) false)
    (Variables|Default|SetbDoArcAdjust false)
    (Variables|/Script/Engine.PrimitiveComponent|SetbGenerateOverlapEvents (Variables|Default|GetPointCollision) false) ; Don't pickup up anything else, youre all done!
    (if (not (Variables|Default|GetbFunnyCollisionMode))
      (Physics|SetSimulatePhysics (Variables|Default|GetPointCollision) false)
      (Collision|SetCollisionEnabled (Variables|Default|GetSkewerMesh) "NoCollision")
      (for _array_element (Variables|Default|GetAttachedFoods)
        (bind _asbp_food_base (Utilities|Casting|CastToBP_FoodBase _array_element))
        (Physics|SetSimulatePhysics (Variables|/Game/Blueprints/BP_FoodBase.BP_FoodBase_C|GetFoodMesh _asbp_food_base) false)
        (Collision|SetCollisionEnabled (Variables|/Game/Blueprints/BP_FoodBase.BP_FoodBase_C|GetFoodMesh _asbp_food_base) "NoCollision"))
      (Variables|Default|SetLastPointValue (CallFunction|GetPointValue))
      (Variables|Default|SetbWallStuck true)
      (Utilities|UpdateWidgetandPop
        (:ExecOut
          (Audio|PlaySoundatLocation "/Game/Audio/WallStab/SC_WallStab1.SC_WallStab1" (Transformation|GetActorLocation) "0, 0, 0" 0.75 (Math|Random|RandomFloatinRange 0.8 1.2) 0.0 0 0 0))))
    (elif (> (Math|Vector|VectorLength _returnvalue_3) 6e+02)
      (bind _hitnormal (Collision|LineTraceComponent OtherComponent _returnvalue (+ _returnvalue (* _returnvalue_2 1e+02)) false false false))
      (if (Math|Float|InRange(Float) (Math|Vector|DotProduct _returnvalue_2 _hitnormal) -1.0 -0.5)
        (goto _label)))))

(fn TryAttachFood
  (params (NewFood :type BP%20Food%20Base%20Object%20Reference))
  (LocalVariables|SetAddFood NewFood)
  (if (and (< (Utilities|Array|Length (Variables|Default|GetAttachedFoods)) (Variables|Default|GetMaxFood)) (not (Utilities|IsValid (Variables|/Game/Blueprints/BP_FoodBase.BP_FoodBase_C|GetSkewerRef (LocalVariables|GetAddFood)))))
    (Default|AttachtoSkewer (LocalVariables|GetAddFood) self)
    (Utilities|Array|AddUnique (Variables|Default|GetAttachedFoods) (LocalVariables|GetAddFood))
    (CallFunction|RefreshFoodPosition)
    (Physics|AddImpulse (Variables|Default|GetSkewerMesh) (* (Math|Vector|GetUpVector (Variables|Default|GetSkewerMesh)) (Variables|Default|GetHitDampen)) "None" false) ; Slow ourselves down a bit
    (Variables|Default|SetLastPointValue (CallFunction|GetPointValue))
    (Utilities|UpdateWidgetandPop
      (:ExecOut
        (Audio|PlaySoundatLocation "/Game/Audio/Foodstab/StabCue.StabCue" (Transformation|GetActorLocation) "0, 0, 0" 0.5 1.0 0.0 0 0 0)))))

(fn RefreshFoodPosition
  (LocalVariables|SetLastPosition (.z (Variables|/Script/Engine.SceneComponent|GetRelativeLocation (Variables|Default|GetFoodPosMin))))
  (for (_array_element _array_index) (Variables|Default|GetAttachedFoods)
    (Transformation|SetActorRelativeLocation _array_element (Math|Vector|MakeVector (* _array_index (LocalVariables|GetForwardSpacing)) 0.0 (LocalVariables|GetLastPosition)))
    (LocalVariables|SetLastPosition (+ (LocalVariables|GetLastPosition) (Variables|Default|GetFoodSpacing)))))

(fn SetAnglebyVelocity
  (params (Delta :type Float%20%28single-precision%29))
  (bind _returnvalue (Physics|GetPhysicsLinearVelocity (Variables|Default|GetSkewerMesh) "None"))
  (if (> (Math|Vector|VectorLength _returnvalue) 8e+02)
    (Transformation|SetActorRotation (Math|Interpolation|RInterpTo (Transformation|GetActorRotation) (Math|Rotator|MakeRotfromZ (Math|Vector|Normalize _returnvalue)) Delta 1e+02))))

(fn GetPointValue
  (for _array_element (Variables|Default|GetAttachedFoods)
    (LocalVariables|SetTotalBasePoints (+ (Variables|/Game/Blueprints/BP_FoodBase.BP_FoodBase_C|GetPointBase _array_element) (LocalVariables|GetTotalBasePoints))))
  (Utilities|FlowControl|Sequence
    (:then_0
      (LocalVariables|SetPointMultiplier (+ (.OutMultiplier (CallFunction|PointCheckFullSkewer)) (LocalVariables|GetPointMultiplier))))
    (:then_1
      (LocalVariables|SetPointMultiplier (+ (.MultiplierOut (CallFunction|PointCheckFullSet)) (LocalVariables|GetPointMultiplier))))
    (:then_2
      (LocalVariables|SetTotalBasePoints (+ (.BaseAdditionOut (CallFunction|PointCheckSetFinish)) (LocalVariables|GetTotalBasePoints))))
    (:then_3
      (LocalVariables|SetPointMultiplier (+ (.MultOut (CallFunction|PointCheckFoodAllSame)) (LocalVariables|GetPointMultiplier))))
    (:then_4
      (LocalVariables|SetPointMultiplier (+ (.MultOut (CallFunction|PointCheckFoodAllDifferent)) (LocalVariables|GetPointMultiplier))))
    (:then_5
      (bind _output_get (LocalVariables|SetFinalPoints (+ (LocalVariables|GetTotalBasePoints) (Math|Float|Round (* (LocalVariables|GetTotalBasePoints) (/ (Math|Conversions|ToFloat(Integer) (LocalVariables|GetPointMultiplier)) 1e+02))))))
      (return (LocalVariables|GetFinalPoints)))))

(fn PointCheckFullSet
  (for _array_element (Variables|Default|GetAttachedFoods) ; FullSet
    (if (not (Utilities|Array|ContainsItem (LocalVariables|GetSkipFoods) _array_element))
      (LocalVariables|SetbFullSet true)
      (bind _array_element_2 (Utilities|Array|ForEachLoopwithBreak (Variables|/Game/Blueprints/BP_FoodBase.BP_FoodBase_C|GetSiblingFoods _array_element) :!label _label)
        (:LoopBody
          (Utilities|Array|AddUnique (LocalVariables|GetSkipFoods) _array_element_2)
          (if (Utilities|IsValid _array_element_2)
            (if (not (== (Variables|/Game/Blueprints/BP_FoodBase.BP_FoodBase_C|GetSkewerRef _array_element_2) self))
              (LocalVariables|SetbFullSet false :!label _label_2)
              (goto _label Break))
            (else
              (goto _label_2))))
        (:Completed
          (if (LocalVariables|GetbFullSet)
            (bind _output_get (LocalVariables|SetReturnMultiplier (+ (LocalVariables|GetReturnMultiplier) (* (+ (Utilities|Array|Length (Variables|/Game/Blueprints/BP_FoodBase.BP_FoodBase_C|GetSiblingFoods _array_element)) 1) 20))))
            (Utilities|Array|Add (LocalVariables|GetFoundFullSets) (+ (Utilities|Array|Length (Variables|/Game/Blueprints/BP_FoodBase.BP_FoodBase_C|GetSiblingFoods _array_element)) 1)))))))
  (return (LocalVariables|GetReturnMultiplier) (LocalVariables|GetFoundFullSets)))

(fn PointCheckSetFinish
  (for _array_element (Variables|Default|GetAttachedFoods) ; FullSet
    (if (not (Utilities|Array|ContainsItem (LocalVariables|GetSkipFoods) _array_element))
      (LocalVariables|SetbSetFinish true)
      (bind _array_element_2 (Utilities|Array|ForEachLoopwithBreak (Variables|/Game/Blueprints/BP_FoodBase.BP_FoodBase_C|GetSiblingFoods _array_element) :!label _label)
        (:LoopBody
          (Utilities|Array|AddUnique (LocalVariables|GetSkipFoods) _array_element_2)
          (if (Utilities|IsValid _array_element_2)
            (if (not (Utilities|IsValid (Variables|/Game/Blueprints/BP_FoodBase.BP_FoodBase_C|GetSkewerRef _array_element_2)))
              (LocalVariables|SetbSetFinish false :!label _label_2)
              (goto _label Break))
            (else
              (goto _label_2))))
        (:Completed
          (if (LocalVariables|GetbSetFinish)
            (bind _output_get (LocalVariables|SetReturnBase (+ (LocalVariables|GetReturnBase) 100)))
            (Math|Integer|IncrementInt (LocalVariables|GetSetCount)))))))
  (return (LocalVariables|GetReturnBase) (LocalVariables|GetSetCount)))

(fn PointCheckFullSkewer
  (bind _attachedfoods (Variables|Default|GetAttachedFoods))
  (bind _maxfood (Variables|Default|GetMaxFood))
  (bind _returnvalue (Utilities|Array|Length _attachedfoods))
  (bind _returnvalue_2 (>= _returnvalue _maxfood))
  (return (Math|Integer|SelectInt 100 0 _returnvalue_2) _returnvalue_2))

(fn PointCheckFoodAllSame
  (if (>= (Utilities|Array|Length (Variables|Default|GetAttachedFoods)) 4)
    (LocalVariables|SetFirstFoodType (Variables|/Game/Blueprints/BP_FoodBase.BP_FoodBase_C|GetFoodType (Utilities|Array|Get(acopy) (Variables|Default|GetAttachedFoods))))
    (LocalVariables|SetbFoodAllSame true)
    (bind _array_element (Utilities|Array|ForEachLoopwithBreak (Variables|Default|GetAttachedFoods) :!label _label)
      (:LoopBody
        (if (not (Utilities|Enum|Equal(Enum) (Variables|/Game/Blueprints/BP_FoodBase.BP_FoodBase_C|GetFoodType _array_element) (LocalVariables|GetFirstFoodType)))
          (LocalVariables|SetbFoodAllSame false)
          (goto _label Break)))
      (:Completed
        (bind _output_get (LocalVariables|SetRetMult (select (LocalVariables|GetbFoodAllSame) (* (Utilities|Array|Length (Variables|Default|GetAttachedFoods)) 10) 0) :!label _label_2))
        (return _output_get (LocalVariables|GetbFoodAllSame))))
    (else
      (goto _label_2))))

(fn PointCheckFoodAllDifferent
  (if (>= (Utilities|Array|Length (Variables|Default|GetAttachedFoods)) 4)
    (LocalVariables|SetbFoodAllDifferent true)
    (bind _array_element (Utilities|Array|ForEachLoopwithBreak (Variables|Default|GetAttachedFoods) :!label _label)
      (:LoopBody
        (if (Utilities|Array|ContainsItem (LocalVariables|GetFoods) (Variables|/Game/Blueprints/BP_FoodBase.BP_FoodBase_C|GetFoodType _array_element))
          (LocalVariables|SetbFoodAllDifferent false)
          (goto _label Break)
          (else
            (Utilities|Array|Add (LocalVariables|GetFoods) (Variables|/Game/Blueprints/BP_FoodBase.BP_FoodBase_C|GetFoodType _array_element)))))
      (:Completed
        (bind _output_get (LocalVariables|SetRetMult (select (LocalVariables|GetbFoodAllDifferent) (* (Utilities|Array|Length (Variables|Default|GetAttachedFoods)) 10) 0) :!label _label_2))
        (return _output_get (LocalVariables|GetbFoodAllDifferent))))
    (else
      (goto _label_2))))