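; LivePlayerData holds the current player's runtime state: identity, XP, unlocked ingredients, seasonings and marinades, plus fridge and food selections.
; Saving copies identity, XP and unlocks into a new SkewerSaveGame, using PlayerName as slot name.
; Loading clears everything before restoring XP and unlocks, but ignores UserName, leaving the slot name empty.
; LoadAndUnlockAll instead fills every unlock list by iterating the type enums.
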(fn LoadSavedData
  (params (UserName :type String) (UserIndex :type Integer))
  (CallFunction|ClearData)
  (Variables|Default|SetPlayerName (Variables|Default|GetPlayerName))
  (Variables|Default|SetUserIndex UserIndex)
  (bind _returnvalue (SaveGame|LoadGamefromSlot (Variables|Default|GetPlayerName) UserIndex))
  (bind _asskewer_save_game (Utilities|Casting|CastToSkewerSaveGame _returnvalue)
    (:then
      (Development|PrintString 0 "Skewer Load Successful")
      (Variables|Default|SetXP (Variables|/Game/Blueprints/SaveGame/SkewerSaveGame.SkewerSaveGame_C|GetXP _asskewer_save_game))
      (Variables|Default|SetUnlockedIngredients (Variables|/Game/Blueprints/SaveGame/SkewerSaveGame.SkewerSaveGame_C|GetUnlockedIngredients _asskewer_save_game))
      (Variables|Default|SetUnlockedSeasonings (Variables|/Game/Blueprints/SaveGame/SkewerSaveGame.SkewerSaveGame_C|GetUnlockedSeasonings _asskewer_save_game))
      (Variables|Default|SetUnlockedMarinades (Variables|/Game/Blueprints/SaveGame/SkewerSaveGame.SkewerSaveGame_C|GetUnlockedMarinades _asskewer_save_game)))
    (:CastFailed
      (Development|PrintString 0 "Skewer Load Failed"))))

(fn SaveCurrentData
  (bind _returnvalue (SaveGame|CreateSaveGameObject "/Game/Blueprints/SaveGame/SkewerSaveGame.SkewerSaveGame_C"))
  (LocalVariables|SetNewSaveGame _returnvalue)
  (Utilities|FlowControl|Sequence
    (:then_0
      (Variables|/Game/Blueprints/SaveGame/SkewerSaveGame.SkewerSaveGame_C|SetPlayerName (LocalVariables|GetNewSaveGame) (Variables|Default|GetPlayerName))
      (Variables|/Game/Blueprints/SaveGame/SkewerSaveGame.SkewerSaveGame_C|SetXP (LocalVariables|GetNewSaveGame) (Variables|Default|GetXP))
      (Variables|/Game/Blueprints/SaveGame/SkewerSaveGame.SkewerSaveGame_C|SetUnlockedIngredients (LocalVariables|GetNewSaveGame) (Variables|Default|GetUnlockedIngredients))
      (Variables|/Game/Blueprints/SaveGame/SkewerSaveGame.SkewerSaveGame_C|SetUnlockedSeasonings (LocalVariables|GetNewSaveGame) (Variables|Default|GetUnlockedSeasonings))
      (Variables|/Game/Blueprints/SaveGame/SkewerSaveGame.SkewerSaveGame_C|SetUnlockedMarinades (LocalVariables|GetNewSaveGame) (Variables|Default|GetUnlockedMarinades)))
    (:then_1
      (SaveGame|SaveGametoSlot 0 (Variables|Default|GetPlayerName) (Variables|Default|GetUserIndex)))))

(fn LoadandUnlockAll
  (params (UserName :type String) (UserIndex :type Integer) (XP :type Integer))
  (CallFunction|ClearData)
  (Variables|Default|SetPlayerName UserName)
  (Variables|Default|SetUserIndex UserIndex)
  (Variables|Default|SetXP XP)
  (Utilities|FlowControl|Sequence
    (:then_0
      (bind _enumvalue (|ForEachFoodType)
        (:LoopBody
          (Utilities|Set|Add (Variables|Default|GetUnlockedIngredients) _enumvalue))))
    (:then_1
      (bind _enumvalue_2 (|ForEachSeasoningType)
        (:LoopBody
          (Utilities|Set|Add (Variables|Default|GetUnlockedSeasonings) _enumvalue_2))))
    (:then_2
      (bind _enumvalue_3 (|ForEachMarinadeType)
        (:LoopBody
          (Utilities|Set|Add (Variables|Default|GetUnlockedMarinades) _enumvalue_3))))))

(fn ClearData
  (Variables|Default|SetPlayerName "")
  (Variables|Default|SetUserIndex 0)
  (Variables|Default|SetXP 0)
  (Utilities|Set|Clear (Variables|Default|GetUnlockedIngredients))
  (Utilities|Set|Clear (Variables|Default|GetUnlockedSeasonings))
  (Utilities|Set|Clear (Variables|Default|GetUnlockedMarinades))
  (Utilities|Array|Clear (Variables|Default|GetFridgeContents))
  (Variables|Default|SetCurrentSeasoning "NewEnumerator2")
  (Variables|Default|SetCurrentMarinade "NewEnumerator2")
  (Utilities|Array|Clear (Variables|Default|GetCurrentFoodSelection)))