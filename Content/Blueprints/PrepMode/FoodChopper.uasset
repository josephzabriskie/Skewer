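; Prep-mode chopping minigame actor: food slides along a track and a timed knife chop stocks the player's fridge.
; A knife timeline event grades the food's offset from center against two thresholds, adds it to player data, spawns two impulse-launched halves and flashes a hit indicator.
; PickFood then chooses a random food, preferring ones with fridge room.
; A chop requested late in the swing is queued to play on finish.
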(event Custom|Chop
  (bind _choptimeline (Variables|Default|GetChopTimeline))
  (if (Variables|Default|GetbCanChop)
    (Variables|Default|SetbCanChop false)
    (bind _knifeangle (Timeline|ChopTimeline PlayFromStart)
      (:Update
        (Transformation|SetRelativeRotation (Variables|Default|GetKnife) (Math|Rotator|MakeRotator 0.0 _knifeangle 0.0) false false))
      (:Finished
        (Variables|Default|SetbCanChop true)
        (if (Variables|Default|GetbQueueChop) ; Play queued chop
          (Variables|Default|SetbQueueChop false)
          (CallFunction|Chop)))
      (:KnifeCheckEvt
        (bind _quality (CallFunction|CheckFoodQuality))
        (Default|AddFridgeQualityFood (CallFunction|GetPlayerData) (Variables|Default|GetCurrentFood) _quality 2)
        (CallFunction|ShowHitIndicator)
        (CallFunction|ChopVisuals)
        (CallFunction|PickFood)))
    (else
      (Variables|Default|SetbQueueChop (> (/ (Components|Timeline|GetPlaybackPosition _choptimeline) (Components|Timeline|GetTimelineLength _choptimeline)) 0.8)) ; Give a little leeway for chop timing
    )))

(event Custom|SetFoodMotion
  (params (bMove :type Boolean))
  (bind _movefood (Variables|Default|GetMoveFood))
  (bind _relativelocation (Variables|/Script/Engine.SceneComponent|GetRelativeLocation _movefood))
  (Variables|Default|SetbFoodInMotion bMove)
  (bind _fooddistance (Timeline|FoodMotion PlayFromStart)
    (:Update
      (Transformation|SetRelativeLocation (Variables|Default|GetMoveFood) (Math|Vector|MakeVector (* _fooddistance (Variables|Default|GetFoodTravelDistance)) (.y _relativelocation) (.z _relativelocation)) false false))))

(event Custom|ShowHitIndicator
  (Transformation|SetWorldLocation (Variables|Default|GetChopHitIndicator) (Transformation|GetWorldLocation (Variables|Default|GetIndicatorLine)) false false)
  (bind _hitindicatorcolor (Timeline|HitIndicatorColor PlayFromStart)
    (:Update
      (Sprite|SetSpriteColor (Variables|Default|GetChopHitIndicator) _hitindicatorcolor) ; Note: Currently the  sprite mat doesn't support transparency
    )))

(event EventBeginPlay
  (CallFunction|SetFoodMotion true)
  (Sprite|SetSpriteColor (Variables|Default|GetChopHitIndicator) "(R=0.000000,G=0.000000,B=0.000000,A=0.000000)")
  (CallFunction|PickFood))

(fn ConstructionScript)

(fn CheckFoodQuality
  (bind _movefood (Variables|Default|GetMoveFood))
  (bind _foodtraveldistance (Variables|Default|GetFoodTravelDistance))
  (bind _relativelocation (Variables|/Script/Engine.SceneComponent|GetRelativeLocation _movefood))
  (bind _returnvalue (Math|Float|SafeDivide (.x _relativelocation) _foodtraveldistance))
  (bind _returnvalue_2 (Math|Float|Absolute(Float) _returnvalue))
  (LocalVariables|SetReturn%20Value "NewEnumerator0")
  (if (< _returnvalue_2 (Variables|Default|GetBestThreshold))
    (LocalVariables|SetReturn%20Value "NewEnumerator2")
    (elif (< _returnvalue_2 (Variables|Default|GetGoodThreshold))
      (LocalVariables|SetReturn%20Value "NewEnumerator1")))
  (return (LocalVariables|GetReturn%20Value)))

(fn SetEnable
  (params (bEnable :type Boolean))
  (Variables|Default|SetbCanChop bEnable))

(fn ChopVisuals
  (bind _movefood (Variables|Default|GetMoveFood))
  (bind _returnvalue (Transformation|GetWorldTransform _movefood))
  (for _index (range 0 1)
    (bind _returnvalue_2 (Game|SpawnActorfromClass "/Game/Blueprints/PrepMode/ChoppedFood.ChoppedFood_C" (Math|Transform|MakeTransform (.location _returnvalue) (.rotation _returnvalue) "0.300000,0.300000,0.300000") "AlwaysSpawn" 0 (Variables|Default|GetCurrentFood) 0))
    (Physics|AddImpulse (Variables|/Game/Blueprints/PrepMode/ChoppedFood.ChoppedFood_C|GetFoodSprite _returnvalue_2) (* (Math|Vector|MakeVector 0.0 (Utilities|Select :Index _index :Option%200 0.707 :Option%201 -0.707) 0.707) (Math|Random|RandomFloatinRange 4e+02 6e+02)) "None" true)
    (Class|PrimitiveComponent|AddAngularImpulseinDegrees (Variables|/Game/Blueprints/PrepMode/ChoppedFood.ChoppedFood_C|GetFoodSprite _returnvalue_2) (Math|Vector|MakeVector (* (select (Math|Random|RandomBool) -1 1) (Math|Random|RandomFloatinRange 5e+02 3e+03)) 0.0 0.0) "None" true)))

(fn PickFood
  (bind _output_get (LocalVariables|SetFoodsWithRoom (Default|GetFridgeFoodswithRoom (CallFunction|GetPlayerData))))
  (bind _output_get_2 (Variables|Default|SetCurrentFood (select (> (Utilities|Array|Length _output_get) 0) (Utilities|Array|Get(acopy) (LocalVariables|GetFoodsWithRoom) (Math|Random|RandomIntegerinRange 0 (Utilities|Array|LastIndex (LocalVariables|GetFoodsWithRoom)))) (Utilities|Enum|ByteToEnumEFoodType (Math|Conversions|ToByte(Integer) (Math|Random|RandomIntegerinRange 0 (- (|GetNumEnumEntries) 1)))))))
  (bind _sprite (CallFunction|GetSpritefromFoodType _output_get_2))
  (Rendering|Components|Sprite|SetSprite (Variables|Default|GetMoveFood) _sprite))