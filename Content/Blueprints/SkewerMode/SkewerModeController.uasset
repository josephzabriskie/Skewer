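; Controller for Skewer Mode, running timed rounds in which the player's bow scores against food from a spawner.
; On begin play it finds the bow pawn and food spawner, creates the HUD, and binds score updates and Play Again.
; Each game resets HUD, score, skewers and food, then counts down before enabling firing and spawning.
; A round-duration timer then disables both and shows the final score overlay.
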(event Custom|_ActivatePlayer
  (EventDispatchers|UnbindEventfromCountdownDone (Variables|/Game/Widgets/SkewerHUD/SkewerHUD.SkewerHUD_C|GetGameStartCountdown (Variables|Default|GetHUDRef)) (delegate Custom|_ActivatePlayer))
  (Default|SetAllowFiring (Variables|ExternalRefs|GetPlayerRef) true)
  (Default|SetEnabled (Variables|ExternalRefs|GetSpawnerRef) true)
  (Utilities|Time|SetTimerbyEvent (delegate Custom|_DeactivatePlayer) (Variables|Default|GetRoundDuration))
  (Default|TimerStart (Variables|/Game/Widgets/SkewerHUD/SkewerHUD.SkewerHUD_C|GetSimpleTimer (Variables|Default|GetHUDRef)) (Math|Float|Truncate (Variables|Default|GetRoundDuration))))

(event Custom|_DeactivatePlayer
  (Default|SetAllowFiring (Variables|ExternalRefs|GetPlayerRef) false)
  (Default|SetEnabled (Variables|ExternalRefs|GetSpawnerRef) false)
  (Default|ShowFinalScoreOverlay (Variables|Default|GetHUDRef) (Variables|/Game/Blueprints/SkewerMode/BP_Bow.BP_Bow_C|GetScore (Variables|ExternalRefs|GetPlayerRef))))

(event Custom|ScoreUpdated
  (params (CurrentScore :type Integer))
  ;[0.3086 1 0.318] BeginPlay
  ;;[1 1 1] Score on Bow changed
  (Default|SetScore (Variables|/Game/Widgets/SkewerHUD/SkewerHUD.SkewerHUD_C|GetScoreDisplay (Variables|Default|GetHUDRef)) CurrentScore))

(event Custom|StartNewGame
  (bind _playerref (Variables|ExternalRefs|GetPlayerRef))
  (bind _hudref (Variables|Default|GetHUDRef))
  (bind _gamestartcountdown (Variables|/Game/Widgets/SkewerHUD/SkewerHUD.SkewerHUD_C|GetGameStartCountdown _hudref))
  ;[1 1 1] Cleanup First
  (Default|FullReset (Variables|Default|GetHUDRef))
  (Default|ClearScore _playerref)
  (Default|CleanUpSkewers _playerref)
  (Default|CleanupFood (Variables|ExternalRefs|GetSpawnerRef))
  ;[1 1 1] Pre-game, bow can't shoot, set spawn mode, disable spawning, start countdown
  (Default|SetAllowFiring (Variables|ExternalRefs|GetPlayerRef) false)
  (Default|SetSpawnMode (Variables|ExternalRefs|GetSpawnerRef) "NewEnumerator1" false)
  (Default|SetEnabled (Variables|ExternalRefs|GetSpawnerRef) false)
  (Default|TimedCountdown _gamestartcountdown 3 "Go!")
  (EventDispatchers|BindEventtoCountdownDone _gamestartcountdown (delegate Custom|_ActivatePlayer))
  (Default|FadeTimer (Variables|/Game/Widgets/SkewerHUD/SkewerHUD.SkewerHUD_C|GetSimpleTimer (Variables|Default|GetHUDRef)) true))

(event Custom|PlayAgain
  ;[0.3086 1 0.318] BeginPlay
  ;;[1 1 1] Play Again
  (CallFunction|StartNewGame))

(event EventBeginPlay
  ;[0.3086 1 0.318] BeginPlay
  (Utilities|FlowControl|Sequence
    (:then_0
      ;;[1 1 1] Get Important Actor References
      (bind _asbp_bow (Utilities|Casting|CastToBP_Bow (Game|Player|GetPlayerPawn 0))
        (:then
          (Variables|ExternalRefs|SetPlayerRef _asbp_bow)
          (bind _returnvalue (Actor|GetActorOfClass "/Game/Blueprints/SkewerMode/BP_FooodSpawner.BP_FooodSpawner_C"))
          (bind _output_get (Variables|ExternalRefs|SetSpawnerRef _returnvalue))
          (Utilities|IsValid _output_get
            (:Is%20Not%20Valid
              (Development|PrintString "Couldn't find FooodSpawner"))))
        (:CastFailed
          (Development|PrintString "Couldn't find player pawn"))))
    (:then_1
      ;;[1 1 1] Count Widget Setup
      (bind _returnvalue_2 (UserInterface|CreateWidget "/Game/Widgets/SkewerHUD/SkewerHUD.SkewerHUD_C"))
      (bind _output_get_2 (Variables|Default|SetHUDRef _returnvalue_2))
      (UserInterface|Viewport|AddtoViewport _output_get_2 0)
      (EventDispatchers|BindEventtoScoreUpdate (Variables|ExternalRefs|GetPlayerRef) (delegate Custom|ScoreUpdated)))
    (:then_2
      ;;[1 1 1] Bind to play again
      (EventDispatchers|BindEventtoPlayAgainPressed (Variables|/Game/Widgets/SkewerHUD/SkewerHUD.SkewerHUD_C|GetFinalScoreOverlay (Variables|Default|GetHUDRef)) (delegate Custom|PlayAgain)))
    (:then_3
      (CallFunction|StartNewGame))))

(fn ConstructionScript)