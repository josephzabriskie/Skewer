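; Food spawner for Skewer mode that spawns BP_Food on a looping timer, as random rain or in lines, with switchable mode and optional auto-start.
; Rain drops randomly rotated food from the upper box.
; Timed lines launch evenly spaced, bouncing food upward from the lower box with staggered delays, linked as siblings.
; Spawned food is tracked for bulk cleanup, but the OnDestroyed binding that would untrack it is unconnected.
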(event Custom|SpawnRandom
  (CallFunction|SpawnRandomFood 1))

(event Custom|SpawnLine
  (CallFunction|SpawnFoodLine (Utilities|RandomFoodNum) (Math|Random|RandomFloatinRange 3e+01 6e+01) false))

(event Custom|SpawnTimerStart
  (bind _returnvalue (Utilities|Time|SetTimerbyEvent (Utilities|Select :Index (Variables|Default|GetSpawnType) :NewEnumerator0 (delegate Custom|SpawnRandom) :NewEnumerator1 (delegate Custom|SpawnLine)) (Utilities|Select :Index (Variables|Default|GetSpawnType) :NewEnumerator0 (Variables|Default|GetRainDelay) :NewEnumerator1 (Variables|Default|GetLineDelay)) true))
  (Variables|Default|SetSpawnTimer _returnvalue))

(event Custom|SpawnTimerStop
  (Utilities|Time|ClearandInvalidateTimerbyHandle (Variables|Default|GetSpawnTimer)))

(event EventBeginPlay
  (Utilities|FlowControl|Sequence
    (:then_0
      (bind _returnvalue (Actor|GetActorOfClass "/Game/Blueprints/SkewerMode/BP_Bow.BP_Bow_C"))
      (Variables|Default|SetBowReference _returnvalue))
    (:then_1
      (if (Variables|Default|GetbAutoStart)
        (CallFunction|SetEnabled true)))))

(fn ConstructionScript)

(fn TrySpawnFood
  (if (< (Utilities|Array|Length (Variables|Default|GetAllCurrentFood)) (Variables|Default|GetMaxFood))
    (CallFunction|SpawnRandomFood)))

(fn SpawnRandomFood
  (params (Amount :type Integer))
  (bind _upperspawnbox (Variables|Default|GetUpperSpawnBox))
  (for _index (range 0 Amount)
    (bind _returnvalue (Game|SpawnActorfromClass "/Game/Blueprints/SkewerMode/BP_Food.BP_Food_C" (Math|Transform|MakeTransform (Math|Random|RandomPointinBoundingBox (Transformation|GetWorldLocation _upperspawnbox) (Variables|/Script/Engine.BoxComponent|GetBoxExtent _upperspawnbox)) (Math|Random|RandomRotator true) "0.300000,0.300000,0.300000") "Undefined" 0 "0.000000,0.000000,0.000000" false 0.0 0 false 0.0 "(INVALID)" 0))
    (CallFunction|TrackNewFood _returnvalue)))

(fn SpawnFoodLine
  (params (NumFoods :type Integer) (Spread :type Float%20%28single-precision%29) (bFromTop :type Boolean))
  (bind _upperspawnbox (Variables|Default|GetUpperSpawnBox))
  (bind _lowerspawnbox (Variables|Default|GetLowerSpawnBox))
  (bind _returnvalue (select bFromTop _upperspawnbox _lowerspawnbox))
  (bind _returnvalue_2 (Components|Box|GetScaledBoxExtent _returnvalue))
  ;[1 1 1] Determine center of spawned food
  (bind _output_get (LocalVariables|SetRadiusOfSpread (/ (* (- NumFoods 1) Spread) 2.0)))
  (bind _output_get_2 (LocalVariables|SetSpreadCenter (Math|Random|RandomPointinBoundingBox (Transformation|GetWorldLocation _returnvalue) (Math|Vector|MakeVector (.x _returnvalue_2) (- (.y _returnvalue_2) (LocalVariables|GetRadiusOfSpread)) (.z _returnvalue_2)))))
  (LocalVariables|SetStartLocation (Math|Vector|MakeVector (.x _output_get_2) (- (.y _output_get_2) _output_get) (.z _output_get_2)))
  (LocalVariables|SetDelay (Math|Random|RandomFloatinRange 0.0 0.06))
  (for _index (range 0 (- NumFoods 1))
    (bind _returnvalue_3 (Game|SpawnActorfromClass "/Game/Blueprints/SkewerMode/BP_Food.BP_Food_C" (Math|Transform|MakeTransform (Math|Vector|MakeVector (.x (LocalVariables|GetStartLocation)) (+ (.y (LocalVariables|GetStartLocation)) (* _index Spread)) (.z (LocalVariables|GetStartLocation))) "0, 0, 0" "0.550000,0.550000,0.550000") "Undefined" 0 (Math|Vector|SelectVector "0, 0, 0" "0, 0,52000.000000" bFromTop) true 3.8e+04 1 (> (LocalVariables|GetDelay) 0.0) (+ (LocalVariables|GetStartDelay) (* _index (LocalVariables|GetDelay))) (Utilities|Enum|ByteToEnumFoodType (Math|Conversions|ToByte(Integer) (Math|Random|RandomIntegerinRange 1 (- (|GetNumEnumEntries) 1)))) 0))
    (CallFunction|TrackNewFood _returnvalue_3)
    (Utilities|Array|Add (LocalVariables|GetFoodSpawnSet) _returnvalue_3))
  (for _array_element (LocalVariables|GetFoodSpawnSet)
    (Default|AddSiblingFoods _array_element (LocalVariables|GetFoodSpawnSet))))

(fn OnFoodDestroy
  (params (DestroyedActor :type Actor%20Object%20Reference))
  (bind _asbp_food (Utilities|Casting|CastToBP_Food DestroyedActor))
  (Utilities|Array|RemoveItem (Variables|Default|GetAllCurrentFood) _asbp_food))

(fn TrackNewFood
  (params (NewFood :type BP%20Food%20Object%20Reference))
  (Utilities|Array|Add (Variables|Default|GetAllCurrentFood) NewFood))

(fn CleanupFood
  (Actor|DestroyActor (Variables|Default|GetAllCurrentFood))
  (Utilities|Array|Clear (Variables|Default|GetAllCurrentFood)))

(fn SetEnabled
  (params (bEnable :type Boolean))
  (bind _output_get (Variables|Default|SetbEnabled bEnable))
  (if _output_get
    (CallFunction|SpawnTimerStart)
    (else
      (CallFunction|SpawnTimerStop))))

(fn SetSpawnMode
  (params (Mode :type SpawnMethod%20Enum :default "NewEnumerator0") (Restart :type Boolean))
  (Variables|Default|SetSpawnType Mode)
  (if Restart
    (CallFunction|SpawnTimerStop)
    (CallFunction|SpawnTimerStart)))