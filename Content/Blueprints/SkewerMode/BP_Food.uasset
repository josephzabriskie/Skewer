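; BP_Food is a physics-driven, skewerable food actor for Skewer mode, taking its sprite from FoodType and base points from a data table.
; On spawn, optionally delayed while hidden, it applies an initial impulse and resets its bounce count.
; Hits add bounce impulses while CanBounce allows; otherwise it greys out, becomes unskewerable and is destroyed after a delay.
; It also tracks its skewer and sibling foods, and can detach and respawn at its original transform.
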(event OnComponentHit(FoodMesh)
  (params (HitComponent :type Primitive%20Component%20Object%20Reference) (OtherActor :type Actor%20Object%20Reference) (OtherComp :type Primitive%20Component%20Object%20Reference) (NormalImpulse :type Vector :default "0, 0, 0") (Hit :type Hit%20Result%20Structure%20%28by%20ref%29))
  (CallFunction|TryBounce NormalImpulse))

(event Custom|ResetTransform
  (CallFunction|DetachfromSkewer)
  (Transformation|SetActorTransform (Variables|Movement|GetOrigTransform))
  (CallFunction|DoSpawnyStuff))

(event Custom|DoSpawnyStuff
  (bind _foodmesh (Variables|Default|GetFoodMesh))
  (bind _foodmesh_2 (Variables|Default|GetFoodMesh))
  (Utilities|FlowControl|Sequence
    (:then_0
      ;[1 1 1] MakeVisible and enable physics again if we delayed this guy
      (if (Variables|Spawn|GetbSpawnDelay)
        (Physics|SetSimulatePhysics _foodmesh true)
        (Rendering|SetVisibility _foodmesh true true)))
    (:then_1
      (if (not (Math|Vector|VectorIsZero (Variables|Movement|GetInitialImpulse)))
        ;[1 1 1] Zero out all velocities
        (Physics|SetPhysicsLinearVelocity _foodmesh_2 "0, 0, 0" false "None")
        (Class|PrimitiveComponent|SetPhysicsAngularVelocityinDegrees _foodmesh_2 "0, 0, 0" false "None")
        (Physics|AddImpulse (Variables|Default|GetFoodMesh) (Variables|Movement|GetInitialImpulse) "None" false)))
    (:then_2
      (Variables|Movement|SetBouncesLeft (Variables|Movement|GetMaxBounces)))))

(event Custom|ScheduleCleanup
  (Variables|Default|SetbCleanUpScheduled true)
  (Sprite|SetSpriteColor (Variables|Default|GetFoodSprite) "(R=0.437500,G=0.437500,B=0.437500,A=1.000000)")
  (Utilities|FlowControl|Delay (Variables|Cleanup|GetCleanupDelay))
  (Actor|DestroyActor))

(event Custom|SetSkewerRef
  (params (Skewer :type Skewer%20Projectile%20Object%20Reference))
  (Variables|Default|SetSkewerRef Skewer))

(event Custom|DetachFromSkewer
  (bind _foodmesh (Variables|Default|GetFoodMesh))
  (Transformation|DetachFromActor "KeepWorld" "KeepWorld" "KeepWorld")
  (Variables|Default|SetSkewerRef 0)
  (Collision|SetCollisionEnabled _foodmesh "QueryAndPhysics")
  (Physics|SetSimulatePhysics _foodmesh true))

(event EventBeginPlay
  (bind _foodtype (Variables|Default|GetFoodType))
  (bind _foodmesh (Variables|Default|GetFoodMesh))
  (bind _returnvalue (Utilities|String|EnumtoString _foodtype))
  (Variables|Movement|SetOrigTransform (Transformation|GetActorTransform))
  (CallFunction|UpdateSpritefromType)
  (bind _returnvalue_2 (Utilities|GetDataTableRow "/Game/Blueprints/Data/FoodDataTable.FoodDataTable" (Utilities|String|StringToName _returnvalue)) ; Set up Points
    (:then
      (Variables|Default|SetPointBase (.basepoints _returnvalue_2))
      (if (and (> (Variables|Spawn|GetSpawnDelayTime) 0.0) (Variables|Spawn|GetbSpawnDelay)) ; Either spawn now or delay
        (Utilities|Time|SetTimerbyEvent (delegate Custom|DoSpawnyStuff) (Variables|Spawn|GetSpawnDelayTime)) ; We're delaying, don't move or show until timer ends
        (Physics|SetSimulatePhysics _foodmesh false)
        (Rendering|SetVisibility _foodmesh false true)
        (else
          (CallFunction|DoSpawnyStuff) ; We're going now, just spawn right away
        )))
    (:RowNotFound
      (Development|PrintString (Utilities|String|Append "Error: No row found for : " _returnvalue) true true "(R=1.000000,G=0.000000,B=0.000000,A=1.000000)" 1e+01))))

(event Collision|EventActorBeginOverlap
  (params (OtherActor :type Actor%20Object%20Reference)))

(event EventTick
  (params (DeltaSeconds :type Float%20%28single-precision%29)))

(fn ConstructionScript)

(fn AddSiblingFoods
  (params (Siblings :type Array%20of%20BP%20Food%20Object%20References))
  (bind _output_get (Variables|Default|SetSiblingFoods Siblings))
  (Utilities|Array|RemoveItem _output_get self))

(fn TryBounce
  (params (BounceDirection :type Vector))
  (if (Variables|Movement|GetbBounce)
    (if (Utilities|CanBounce)
      (Physics|AddImpulse (Variables|Default|GetFoodMesh) (* (Math|Vector|Normalize BounceDirection) (Variables|Movement|GetBounceImpulseMagnitude)) "None" false)
      (Math|Integer|DecrementInt (Variables|Movement|GetBouncesLeft))
      (else
        (CallFunction|ScheduleCleanup)))))

(fn CanbeSkewered
  (return (and (not (Utilities|IsValid (Variables|Default|GetSkewerRef))) (not (Variables|Default|GetbCleanUpScheduled)))))

(fn UpdateSpritefromType
  (Rendering|Components|Sprite|SetSprite (Variables|Default|GetFoodSprite) (CallFunction|GetSpritefromFoodType (Variables|Default|GetFoodType))))