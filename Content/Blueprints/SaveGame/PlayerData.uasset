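; PlayerData is the player's SaveGame object, storing name, XP, unlocked ingredients, seasonings and marinades, food selection and fridge stock.
; The fridge maps each food to counts in three quality tiers, spending the best first and trimming the worst when the total exceeds FridgeLevel.
; XP and fridge changes save immediately to a slot named after the player.
; UnlockAll resets the profile with everything unlocked and random stock, while ActivateSeasoningAbility is empty.
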(fn SaveCurrentData
  (SaveGame|SaveGametoSlot self (Variables|Default|GetPlayerName) (Variables|Default|GetUserIndex)))

(fn UnlockAll
  (params (UserName :type String) (UserIndex :type Integer) (NewXP :type Integer))
  (CallFunction|ClearData)
  (Variables|Default|SetPlayerName UserName)
  (Variables|Default|SetUserIndex UserIndex)
  (Variables|Default|SetXP NewXP)
  (Variables|Default|SetFridgeLevel 10)
  (Variables|Default|SetCurrentFoodSelection (Utilities|Array|MakeArray "NewEnumerator0" "NewEnumerator1" "NewEnumerator4" "NewEnumerator9"))
  (Utilities|FlowControl|Sequence
    (:then_0
      (bind _enumvalue (|ForEachEFoodType)
        (:LoopBody
          (Utilities|Set|Add (Variables|Default|GetUnlockedIngredients) _enumvalue))))
    (:then_1
      (bind _enumvalue_2 (|ForEachESeasoningType)
        (:LoopBody
          (Utilities|Set|Add (Variables|Default|GetUnlockedSeasonings) _enumvalue_2))))
    (:then_2
      (bind _enumvalue_3 (|ForEachEMarinadeType)
        (:LoopBody
          (Utilities|Set|Add (Variables|Default|GetUnlockedMarinades) _enumvalue_3))))
    (:then_3
      ;[0.1198 0.1198 0.1198] Fill in fridge
      (bind _result (Utilities|Set|ToArray (Variables|Default|GetUnlockedIngredients)))
      (for _array_element _result
        (Utilities|Map|Add (Variables|Default|GetFridgeContents) _array_element (Utilities|Struct|MakeFridgeEntry _array_element (Math|Random|RandomIntegerinRange 0 4) (Math|Random|RandomIntegerinRange 0 4) (Math|Random|RandomIntegerinRange 0 4)))))
    (:then_4
      (CallFunction|SaveCurrentData))))

(fn ClearData
  (Variables|Default|SetPlayerName "")
  (Variables|Default|SetUserIndex 0)
  (Variables|Default|SetXP 0)
  (Utilities|Set|Clear (Variables|Default|GetUnlockedIngredients))
  (Utilities|Set|Clear (Variables|Default|GetUnlockedSeasonings))
  (Utilities|Set|Clear (Variables|Default|GetUnlockedMarinades))
  (Utilities|Map|Clear (Variables|Default|GetFridgeContents))
  (Utilities|Array|Clear (Variables|Default|GetCurrentFoodSelection))
  (Variables|Default|SetFridgeLevel 0))

(fn AddExperience
  (params (XPAdd :type Integer))
  (Variables|Default|SetXP (+ XPAdd (Variables|Default|GetXP)))
  (CallFunction|SaveCurrentData))

(fn GetFridgeFoodTypes
  (bind _keys (Utilities|Map|Keys (Variables|Default|GetFridgeContents)))
  (return _keys))

(fn UseFridgeFood
  (params (Food :type EFoodType%20Enum :default "NewEnumerator0"))
  (LocalVariables|SetFoodBestQuality (CallFunction|GetFridgeFoodBestQuality Food))
  (LocalVariables|SetFridgeEntry (.Value (Utilities|Map|Find (Variables|Default|GetFridgeContents) Food)))
  (switch Utilities|FlowControl|Switch|SwitchonEFoodQuality (LocalVariables|GetFoodBestQuality)
    (:NewEnumerator3
      _)
    (:NewEnumerator0
      (Utilities|Struct|SetmembersinFridgeEntry (LocalVariables|GetFridgeEntry) (Math|Integer|Max(Integer) (- (Utilities|Select :Index (LocalVariables|GetFoodBestQuality) :NewEnumerator3 0 :NewEnumerator0 (.OKQualityCount (Utilities|Struct|BreakFridgeEntry (LocalVariables|GetFridgeEntry))) :NewEnumerator1 (.GoodQualityCount (Utilities|Struct|BreakFridgeEntry (LocalVariables|GetFridgeEntry))) :NewEnumerator2 (.BestQualityCount (Utilities|Struct|BreakFridgeEntry (LocalVariables|GetFridgeEntry)))) 1)))
      (Utilities|Map|Add (Variables|Default|GetFridgeContents) Food (LocalVariables|GetFridgeEntry) :!label _label)
      (CallFunction|SaveCurrentData))
    (:NewEnumerator1
      (Utilities|Struct|SetmembersinFridgeEntry (LocalVariables|GetFridgeEntry) (Math|Integer|Max(Integer) (- (Utilities|Select :Index (LocalVariables|GetFoodBestQuality) :NewEnumerator3 0 :NewEnumerator0 (.OKQualityCount (Utilities|Struct|BreakFridgeEntry (LocalVariables|GetFridgeEntry))) :NewEnumerator1 (.GoodQualityCount (Utilities|Struct|BreakFridgeEntry (LocalVariables|GetFridgeEntry))) :NewEnumerator2 (.BestQualityCount (Utilities|Struct|BreakFridgeEntry (LocalVariables|GetFridgeEntry)))) 1)))
      (goto _label))
    (:NewEnumerator2
      (Utilities|Struct|SetmembersinFridgeEntry (LocalVariables|GetFridgeEntry) (Math|Integer|Max(Integer) (- (Utilities|Select :Index (LocalVariables|GetFoodBestQuality) :NewEnumerator3 0 :NewEnumerator0 (.OKQualityCount (Utilities|Struct|BreakFridgeEntry (LocalVariables|GetFridgeEntry))) :NewEnumerator1 (.GoodQualityCount (Utilities|Struct|BreakFridgeEntry (LocalVariables|GetFridgeEntry))) :NewEnumerator2 (.BestQualityCount (Utilities|Struct|BreakFridgeEntry (LocalVariables|GetFridgeEntry)))) 1)))
      (goto _label)))
  (return (LocalVariables|GetFoodBestQuality)))

(fn GetFridgeFoodBestQuality
  (params (Food :type EFoodType%20Enum :default "NewEnumerator0"))
  (bind _fridgecontents (Variables|Default|GetFridgeContents))
  (bind (_value _returnvalue) (Utilities|Map|Find _fridgecontents Food))
  (bind (_foodtype _okqualitycount _goodqualitycount _bestqualitycount) (Utilities|Struct|BreakFridgeEntry _value))
  (if _returnvalue
    (if (> _bestqualitycount 0)
      (return "NewEnumerator2")
      (elif (> _goodqualitycount 0)
        (return "NewEnumerator1")
        (elif (> _okqualitycount 0)
          (return "NewEnumerator0")
          (else
            (return "NewEnumerator3")))))
    (else
      (return "NewEnumerator3"))))

(fn AddFridgeQualityFood
  (params (NewFood :type EFoodType%20Enum :default "NewEnumerator0") (NewQuality :type EFoodQuality%20Enum :default "NewEnumerator3") (Amount :type Integer))
  (if (not (or (Utilities|Enum|Equal(Enum) NewQuality "NewEnumerator3") (not (Utilities|Map|Contains (Variables|Default|GetFridgeContents) NewFood))))
    (LocalVariables|SetFridgeEntry (.Value (Utilities|Map|Find (Variables|Default|GetFridgeContents) NewFood)))
    (switch Utilities|FlowControl|Switch|SwitchonEFoodQuality NewQuality
      (:NewEnumerator3)
      (:NewEnumerator0
        (Utilities|Struct|SetmembersinFridgeEntry (LocalVariables|GetFridgeEntry) (Math|Integer|Min(Integer) (+ (Utilities|Select :Index NewQuality :NewEnumerator3 0 :NewEnumerator0 (.OKQualityCount (Utilities|Struct|BreakFridgeEntry (LocalVariables|GetFridgeEntry))) :NewEnumerator1 (.GoodQualityCount (Utilities|Struct|BreakFridgeEntry (LocalVariables|GetFridgeEntry))) :NewEnumerator2 (.BestQualityCount (Utilities|Struct|BreakFridgeEntry (LocalVariables|GetFridgeEntry)))) Amount) (Variables|Default|GetFridgeLevel))))
      (:NewEnumerator1
        (Utilities|Struct|SetmembersinFridgeEntry (LocalVariables|GetFridgeEntry) (Math|Integer|Min(Integer) (+ (Utilities|Select :Index NewQuality :NewEnumerator3 0 :NewEnumerator0 (.OKQualityCount (Utilities|Struct|BreakFridgeEntry (LocalVariables|GetFridgeEntry))) :NewEnumerator1 (.GoodQualityCount (Utilities|Struct|BreakFridgeEntry (LocalVariables|GetFridgeEntry))) :NewEnumerator2 (.BestQualityCount (Utilities|Struct|BreakFridgeEntry (LocalVariables|GetFridgeEntry)))) Amount) (Variables|Default|GetFridgeLevel))))
      (:NewEnumerator2
        (Utilities|Struct|SetmembersinFridgeEntry (LocalVariables|GetFridgeEntry) (Math|Integer|Min(Integer) (+ (Utilities|Select :Index NewQuality :NewEnumerator3 0 :NewEnumerator0 (.OKQualityCount (Utilities|Struct|BreakFridgeEntry (LocalVariables|GetFridgeEntry))) :NewEnumerator1 (.GoodQualityCount (Utilities|Struct|BreakFridgeEntry (LocalVariables|GetFridgeEntry))) :NewEnumerator2 (.BestQualityCount (Utilities|Struct|BreakFridgeEntry (LocalVariables|GetFridgeEntry)))) Amount) (Variables|Default|GetFridgeLevel)))))
    (Utilities|Map|Add (Variables|Default|GetFridgeContents) NewFood (LocalVariables|GetFridgeEntry))
    (CallFunction|TrimFridgeEntry NewFood)
    (CallFunction|SaveCurrentData)
    (Default|CallFridgeUpdated NewFood (.Value (Utilities|Map|Find (Variables|Default|GetFridgeContents) NewFood)))))

(fn GetFridgeFoodEntry
  (params (FoodType :type EFoodType%20Enum :default "NewEnumerator0"))
  (bind _fridgecontents (Variables|Default|GetFridgeContents))
  (bind (_value _returnvalue) (Utilities|Map|Find _fridgecontents FoodType))
  (return _returnvalue _value))

(fn GetSeasonings
  (bind _result (Utilities|Set|ToArray (Variables|Default|GetUnlockedSeasonings)))
  (return _result))

(fn GetMarinades
  (bind _result (Utilities|Set|ToArray (Variables|Default|GetUnlockedMarinades)))
  (return _result))

(fn GetFridgeFoodswithRoom
  (bind _keys (Utilities|Map|Keys (Variables|Default|GetFridgeContents)))
  (for _array_element _keys
    (if (.ReturnValue (Utilities|Map|Find (Variables|Default|GetFridgeContents) _array_element))
      (if (< (.bestqualitycount (.Value (Utilities|Map|Find (Variables|Default|GetFridgeContents) _array_element))) (Variables|Default|GetFridgeLevel))
        (Utilities|Array|Add (LocalVariables|GetOutFoods) _array_element))))
  (return (LocalVariables|GetOutFoods)))

(fn TrimFridgeEntry
  (params (FoodToTrim :type EFoodType%20Enum :default "NewEnumerator0"))
  (bind _fridgecontents (Variables|Default|GetFridgeContents))
  (bind (_value _returnvalue) (Utilities|Map|Find _fridgecontents FoodToTrim))
  (if _returnvalue
    (bind _output_get (LocalVariables|SetEntry _value))
    (bind _output_get_2 (LocalVariables|SetReduceFood (- (+ (.BestQualityCount (Utilities|Struct|BreakFridgeEntry _output_get)) (.GoodQualityCount (Utilities|Struct|BreakFridgeEntry _output_get)) (.OKQualityCount (Utilities|Struct|BreakFridgeEntry _output_get))) (Variables|Default|GetFridgeLevel))))
    (if (> _output_get_2 0)
      ;[0.2188 0.2188 0.2188] Subtract low quality
      (if (>= (.OKQualityCount (Utilities|Struct|BreakFridgeEntry (LocalVariables|GetEntry))) (LocalVariables|GetReduceFood))
        (Utilities|Struct|SetmembersinFridgeEntry (LocalVariables|GetEntry) (- (.OKQualityCount (Utilities|Struct|BreakFridgeEntry (LocalVariables|GetEntry))) (LocalVariables|GetReduceFood)))
        (Utilities|Map|Add (Variables|Default|GetFridgeContents) FoodToTrim (LocalVariables|GetEntry) :!label _label)
        (CallFunction|SaveCurrentData)
        (else
          (LocalVariables|SetReduceFood (- (LocalVariables|GetReduceFood) (.OKQualityCount (Utilities|Struct|BreakFridgeEntry (LocalVariables|GetEntry)))))
          (Utilities|Struct|SetmembersinFridgeEntry (LocalVariables|GetEntry))
          ;[0.2188 0.2188 0.2188] Subtract Medium Quality
          (if (>= (.GoodQualityCount (Utilities|Struct|BreakFridgeEntry (LocalVariables|GetEntry))) (LocalVariables|GetReduceFood))
            (Utilities|Struct|SetmembersinFridgeEntry (LocalVariables|GetEntry) (- (.GoodQualityCount (Utilities|Struct|BreakFridgeEntry (LocalVariables|GetEntry))) (LocalVariables|GetReduceFood)))
            (goto _label)
            (else
              (LocalVariables|SetReduceFood (- (LocalVariables|GetReduceFood) (.GoodQualityCount (Utilities|Struct|BreakFridgeEntry (LocalVariables|GetEntry)))))
              (Utilities|Struct|SetmembersinFridgeEntry (LocalVariables|GetEntry))
              ;[0.2188 0.2188 0.2188] Subtract High Quality
              (if (>= (.BestQualityCount (Utilities|Struct|BreakFridgeEntry (LocalVariables|GetEntry))) (LocalVariables|GetReduceFood))
                (Utilities|Struct|SetmembersinFridgeEntry (LocalVariables|GetEntry) (- (.BestQualityCount (Utilities|Struct|BreakFridgeEntry (LocalVariables|GetEntry))) (LocalVariables|GetReduceFood)))
                (goto _label)
                (else
                  (LocalVariables|SetReduceFood (- (LocalVariables|GetReduceFood) (.BestQualityCount (Utilities|Struct|BreakFridgeEntry (LocalVariables|GetEntry)))))
                  (Utilities|Struct|SetmembersinFridgeEntry (LocalVariables|GetEntry))
                  (if (> (LocalVariables|GetReduceFood) 0)
                    (Development|PrintString 0 (Utilities|String|Append "Somehow we didn't remove enough: " (Utilities|String|ToString(Integer) (LocalVariables|GetReduceFood))))
                    (goto _label)))))))))))

(fn GetFoodSelection
  (params (Index :type Integer))
  (return (Utilities|Array|Get(acopy) (Variables|Default|GetCurrentFoodSelection) Index)))

(fn GetAllFoodSelections
  (return (Variables|Default|GetCurrentFoodSelection)))

(fn SetFoodSelection
  (params (Index :type Integer) (FoodType :type EFoodType%20Enum :default "NewEnumerator0"))
  (Utilities|Array|SetArrayElem (Variables|Default|GetCurrentFoodSelection) Index FoodType))

(fn ActivateSeasoningAbility
  (params (Seasoning :type ESeasoningType%20Enum :default "NewEnumerator2")))