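; Blueprint function library of shared helpers for the skewer game.
; It maps each food type, from meats and fish to vegetables, cheese and lemon, to its sprite through a single Select.
; It also fetches the game instance cast to SkewerGameInstance, and builds on that getter to return the LivePlayerData stored there.
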(fn GetSpritefromFoodType
  (params (FoodType :type EFoodType%20Enum :default "NewEnumerator14"))
  (return (Utilities|Select :Index FoodType :NewEnumerator0 "/Game/Textures/Bodies/Meat_Cube_Sprite.Meat_Cube_Sprite" :NewEnumerator1 "/Game/Textures/Bodies/Chicken_Sprite.Chicken_Sprite" :NewEnumerator13 "/Game/Textures/Bodies/Fish_Sprite.Fish_Sprite" :NewEnumerator4 "/Game/Textures/Bodies/Red_Onion_Sprite.Red_Onion_Sprite" :NewEnumerator5 "/Game/Textures/Bodies/Red_Pepper_Sprite.Red_Pepper_Sprite" :NewEnumerator6 "/Game/Textures/Bodies/Green_Pepper_Sprite.Green_Pepper_Sprite" :NewEnumerator8 "/Game/Textures/Bodies/Tomato_Sprite.Tomato_Sprite" :NewEnumerator9 "/Game/Textures/Bodies/Mushroom_Sprite.Mushroom_Sprite" :NewEnumerator10 "/Game/Textures/Bodies/Green_Zucchini_Sprite.Green_Zucchini_Sprite" :NewEnumerator11 "/Game/Textures/Bodies/Cheese_Sprite.Cheese_Sprite" :NewEnumerator12 "/Game/Textures/Bodies/Lemon_Sprite.Lemon_Sprite" :NewEnumerator16 "/Game/Textures/Bodies/Potato_Sprite.Potato_Sprite" :NewEnumerator17 "/Game/Textures/Bodies/Yellow_Zucchini_Sprite.Yellow_Zucchini_Sprite" :NewEnumerator18 "/Game/Textures/Bodies/Onion_Sprite.Onion_Sprite")))

(fn GetSkewerGameInstance
  (return (.AsSkewer%20Game%20Instance (Utilities|Casting|CastToSkewerGameInstance (Game|GetGameInstance (LocalVariables|Get__WorldContext))))))

(fn GetPlayerData
  (return (Variables|/Game/Blueprints/SkewerGameInstance.SkewerGameInstance_C|GetLivePlayerData (CallFunction|GetSkewerGameInstance (LocalVariables|Get__WorldContext)))))