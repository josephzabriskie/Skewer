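; Base ability Blueprint providing timer-driven activation, duration and cooldown logic, with duration and cooldown getters meant for child overrides.
; ActivateAbility starts a duration timer only when Ready, but does not set Active.
; HandleTimerEvent resets Active or Cooldown to Ready through SetState, which fires a state-change call, and starts a cooldown timer from Active.
; GetCurrentTimer gives remaining time only while Active and always reports Ready.
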(event EventBeginPlay)

(event Collision|EventActorBeginOverlap
  (params (OtherActor :type Actor%20Object%20Reference)))

(event EventTick
  (params (DeltaSeconds :type Float%20%28single-precision%29)))

(fn ConstructionScript)

(fn HandleTimerEvent
  (switch Utilities|FlowControl|Switch|SwitchonEAbilityState (Variables|Default|GetCurrentState)
    (:NewEnumerator0
      (Development|PrintString "We shouldn't have set a timer when in state Ready"))
    (:NewEnumerator1
      (CallFunction|SetState "NewEnumerator0")
      (bind _outcooldown (CallFunction|GetMaxCooldown))
      (bind _returnvalue (Utilities|Time|SetTimerbyEvent (EventDispatchers|CreateEvent :!event HandleTimerEvent) (Math|Timespan|GetTotalSeconds _outcooldown)))
      (Variables|Default|SetTimerHandle _returnvalue))
    (:NewEnumerator2
      (CallFunction|SetState "NewEnumerator0"))))

(fn ActivateAbility
  (if (Utilities|Enum|Equal(Enum) (Variables|Default|GetCurrentState) "NewEnumerator0")
    (bind _outduration (CallFunction|GetMaxDuration))
    (bind _returnvalue (Utilities|Time|SetTimerbyEvent (EventDispatchers|CreateEvent :!event HandleTimerEvent) (Math|Timespan|GetTotalSeconds _outduration)))
    (Variables|Default|SetTimerHandle _returnvalue)
    (return true)
    (else
      (return false))))

(fn GetMaxDuration
  (Development|PrintString "Error: this should be overriden")
  (return ""))

(fn GetCurrentTimer
  (bind _timerhandle (Variables|Default|GetTimerHandle))
  (bind _returnvalue (Utilities|Time|GetTimerRemainingTimebyHandle _timerhandle))
  (if (and (Utilities|Time|IsTimerActivebyHandle (Variables|Default|GetTimerHandle)) (Utilities|Enum|Equal(Enum) (Variables|Default|GetCurrentState) "NewEnumerator1"))
    (LocalVariables|SetReturnTimespan (Math|Timespan|MakeTimespan 0 0 0 (Math|Float|Truncate _returnvalue) (Math|Float|Truncate (* 1000 (Math|Float|Fraction _returnvalue)))))
    (else
      (LocalVariables|SetReturnTimespan (Math|Timespan|MakeTimespan 0))))
  (return (LocalVariables|GetReturnTimespan) "NewEnumerator0"))

(fn GetMaxCooldown
  (Development|PrintString "Error: this should be overriden")
  (return ""))

(fn SetState
  (params (NewState :type EAbilityState%20Enum :default "NewEnumerator0"))
  (bind _output_get (Variables|Default|SetCurrentState NewState))
  (Default|CallAbilityStateChange _output_get))