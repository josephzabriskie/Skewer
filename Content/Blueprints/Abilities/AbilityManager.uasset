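; Manager that owns the player's Seasoning and Marinade abilities and handles their activation, state queries and resets.
; InitAbilities builds one Ability object per enum value, linked to its data table row by enum name, into a map per type.
; Activating an ability first deactivates others of the same type, keeping one active per type.
; Save data is gathered from every ability and reapplied only once initialization is done.
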(fn InitAbilities
  (Variables|Default|SetbAbilitiesInit true)
  ;[1 1 1] ResetSeasonings
  (Utilities|Map|Clear (Variables|Default|GetSeasoningAbilities))
  (bind _enumvalue (|ForEachESeasoningType)
    (:LoopBody
      (bind _returnvalue (Game|ConstructObjectfromClass "/Game/Blueprints/Abilities/Ability.Ability_C" self "NewEnumerator0" _enumvalue "/Game/Blueprints/Data/SeasoningAbilities.SeasoningAbilities" (Utilities|String|StringToName (Utilities|String|EnumtoString _enumvalue))))
      (Utilities|Map|Add (Variables|Default|GetSeasoningAbilities) _enumvalue _returnvalue))
    (:then
      ;[1 1 1] Reset Marinades
      (Utilities|Map|Clear (Variables|Default|GetMarinadeAbilities))
      (bind _enumvalue_2 (|ForEachEMarinadeType)
        (:LoopBody
          (bind _returnvalue_2 (Game|ConstructObjectfromClass "/Game/Blueprints/Abilities/Ability.Ability_C" self "NewEnumerator1" _enumvalue_2 "/Game/Blueprints/Data/MarinadeAbilities.MarinadeAbilities" (Utilities|String|StringToName (Utilities|String|EnumtoString _enumvalue_2))))
          (Utilities|Map|Add (Variables|Default|GetMarinadeAbilities) _enumvalue_2 _returnvalue_2))))))

(fn AbilityInitDone
  (return (Variables|Default|GetbAbilitiesInit)))

(fn ActivateAbility
  (params (AbilityType :type EAbilityType%20Enum :default "NewEnumerator0") (AbilityEnum :type Byte))
  (bind _output_get (LocalVariables|SetAbilityRef (CallFunction|GetAbility AbilityType AbilityEnum)))
  (if (Utilities|IsValid _output_get)
    (CallFunction|DeactivateAll AbilityType) ; Only allow one seasoning active at a time
    (bind _bsuccess (Default|ActivateAbility (LocalVariables|GetAbilityRef)))
    (Default|CallAbilityActivated AbilityType AbilityEnum)
    (return _bsuccess)
    (else
      (Development|PrintString (Utilities|String|Append (Utilities|String|EnumtoString AbilityType) " Not found: " (Utilities|String|ToString(Byte) AbilityEnum)))
      (return false))))

(fn DeactivateAbility
  (params (AbilityType :type EAbilityType%20Enum :default "NewEnumerator0") (AbilityEnum :type Byte))
  (bind _output_get (LocalVariables|SetAbilityRef (CallFunction|GetAbility AbilityType AbilityEnum)))
  (if (Utilities|IsValid _output_get)
    (bind _bsuccess (Default|DeactivateAbility (LocalVariables|GetAbilityRef)))
    (return _bsuccess)
    (else
      (Development|PrintString (Utilities|String|Append (Utilities|String|EnumtoString AbilityType) " Not found: " (Utilities|String|ToString(Byte) AbilityEnum)))
      (return false))))

(fn DeactivateAll
  (params (AbilityType :type EAbilityType%20Enum :default "NewEnumerator0"))
  (if (Utilities|Enum|Equal(Enum) AbilityType "NewEnumerator0")
    (bind _keys (Utilities|Map|Keys (Variables|Default|GetSeasoningAbilities)))
    (for _array_element _keys
      (Utilities|IsValid (.Value (Utilities|Map|Find (Variables|Default|GetSeasoningAbilities) _array_element))
        (:Is%20Valid
          (if (Default|IsActive (.Value (Utilities|Map|Find (Variables|Default|GetSeasoningAbilities) _array_element)))
            (Development|PrintString (Utilities|String|Append "Deactivated: " (Utilities|String|EnumtoString _array_element)))
            (bind _bsuccess (Default|DeactivateAbility (.Value (Utilities|Map|Find (Variables|Default|GetSeasoningAbilities) _array_element))))
            (if (not _bsuccess)
              (Development|PrintString (Utilities|String|Append "Error: Deactivating seasoning failed: " (Utilities|String|EnumtoString _array_element))))))))
    (else
      (bind _keys_2 (Utilities|Map|Keys (Variables|Default|GetMarinadeAbilities)))
      (for _array_element_2 _keys_2
        (Utilities|IsValid (.Value (Utilities|Map|Find (Variables|Default|GetMarinadeAbilities) _array_element_2))
          (:Is%20Valid
            (if (Default|IsActive (.Value (Utilities|Map|Find (Variables|Default|GetMarinadeAbilities) _array_element_2)))
              (Development|PrintString (Utilities|String|Append "Deactivated: " (Utilities|String|EnumtoString _array_element_2)))
              (bind _bsuccess_2 (Default|DeactivateAbility (.Value (Utilities|Map|Find (Variables|Default|GetMarinadeAbilities) _array_element_2))))
              (if (not _bsuccess_2)
                (Development|PrintString (Utilities|String|Append "Error: Deactivating Marinade failed: " (Utilities|String|EnumtoString _array_element_2)))))))))))

(fn GetAbilityState
  (params (AbilityType :type EAbilityType%20Enum :default "NewEnumerator0") (AbilityEnum :type Byte))
  (bind _output_get (LocalVariables|SetAbilityRef (CallFunction|GetAbility AbilityType AbilityEnum)))
  (if (Utilities|IsValid _output_get)
    (return (.AbilityState (Default|GetState (LocalVariables|GetAbilityRef))) (.OutTimspan (Default|GetState (LocalVariables|GetAbilityRef))))
    (else
      (Development|PrintString "Error: No ability found to get info from")
      (return "NewEnumerator0" ""))))

(fn GetAbility
  (params (AbilityType :type EAbilityType%20Enum :default "NewEnumerator0") (AbilityEnum :type Byte))
  (return (.Value (Utilities|Map|Find (CallFunction|GetAbilityDict AbilityType) AbilityEnum))))

(fn GetActiveAbility
  (params (AbilityType :type EAbilityType%20Enum :default "NewEnumerator0"))
  (bind _outdict (CallFunction|GetAbilityDict AbilityType))
  (bind _abilities (CallFunction|GetAllAbilitiesinState "NewEnumerator1" _outdict))
  (bind _returnvalue (Utilities|Array|Length _abilities))
  (if (> _returnvalue 0)
    (if (> _returnvalue 1)
      (Development|PrintString "Why are more than 1 abilities active?") ; Shouldn't happen!
    )
    (return (Utilities|Array|Get(acopy) _abilities))
    (else
      (return 0))))

(fn GetCooldownAbilities
  (params (AbilityType :type EAbilityType%20Enum :default "NewEnumerator0"))
  (return (CallFunction|GetAllAbilitiesinState "NewEnumerator2" (CallFunction|GetAbilityDict AbilityType))))

(fn SetbySaveData
  (params (SavedData :type Array%20of%20Ability%20Save%20Data%20Structures))
  (if (CallFunction|AbilityInitDone)
    (for _array_element SavedData
      (Default|SetbySaveData (CallFunction|GetAbility (.AbilityType (Utilities|Struct|BreakAbilitySaveData _array_element)) (.AbilityEnum (Utilities|Struct|BreakAbilitySaveData _array_element))) _array_element))
    (else
      (Development|PrintString "Couldn't set abilities by Save Data. Init Not done yet"))))

(fn GetSaveData
  (bind _enumvalue (|ForEachESeasoningType) ; Seasonings
    (:LoopBody
      (Utilities|Array|Add (LocalVariables|GetOutArray) (Default|GetSaveData (CallFunction|GetAbility "NewEnumerator0" _enumvalue))))
    (:then
      (bind _enumvalue_2 (|ForEachEMarinadeType) ; marinades
        (:LoopBody
          (Utilities|Array|Add (LocalVariables|GetOutArray) (Default|GetSaveData (CallFunction|GetAbility "NewEnumerator1" _enumvalue_2))))
        (:then
          (return (LocalVariables|GetOutArray)))))))

(fn GetAllAbilitiesinState
  (params (AbilityState :type EAbilityState%20Enum :default "NewEnumerator0") (AbilityDict :type Map%20of%20Bytes%20to%20Objects))
  (bind _keys (Utilities|Map|Keys AbilityDict))
  (for _array_element _keys
    (if (Utilities|Enum|Equal(Enum) (.AbilityState (Default|GetState (.Value (Utilities|Map|Find AbilityDict _array_element)))) AbilityState)
      (Utilities|Array|Add (LocalVariables|GetOutAbilities) (.Value (Utilities|Map|Find AbilityDict _array_element)))))
  (return (LocalVariables|GetOutAbilities)))

(fn GetAbilityDict
  (params (AbilityType :type EAbilityType%20Enum :default "NewEnumerator0"))
  (switch Utilities|FlowControl|Switch|SwitchonEAbilityType AbilityType
    (:NewEnumerator0
      (LocalVariables|SetAbilityDict (Variables|Default|GetSeasoningAbilities)))
    (:NewEnumerator1
      (LocalVariables|SetAbilityDict (Variables|Default|GetMarinadeAbilities))))
  (return (LocalVariables|GetAbilityDict)))

(fn ResetAbilitiesOfType
  (params (Type :type EAbilityType%20Enum :default "NewEnumerator0"))
  (Utilities|FlowControl|Sequence
    (:then_0
      (switch Utilities|FlowControl|Switch|SwitchonEAbilityType Type
        (:NewEnumerator0
          (bind _values (Utilities|Map|Values (Variables|Default|GetSeasoningAbilities)))
          (LocalVariables|SetAbilitiesToReset _values))
        (:NewEnumerator1
          (bind _values_2 (Utilities|Map|Values (Variables|Default|GetMarinadeAbilities)))
          (LocalVariables|SetAbilitiesToReset _values_2))))
    (:then_1
      (for _array_element (LocalVariables|GetAbilitiesToReset)
        (Default|ForceReset _array_element)))))