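; Ability Blueprint that runs a single ability through Ready, Active and Cooldown states on one timer handle.
; Duration and cooldown come from a data table row named from the ability type and enum.
; Activation starts the duration timer, whose expiry leads into cooldown and then Ready, while early deactivation adds remaining active time to the cooldown.
; State changes are broadcast through AbilityStateChange, and GetState reports remaining time as a Timespan.
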(fn ActivateAbility
  (if (Utilities|Enum|Equal(Enum) (Variables|Default|GetCurrentState) "NewEnumerator0")
    (bind _outduration (CallFunction|GetMaxDuration))
    (bind _returnvalue (Utilities|Time|SetTimerbyEvent (EventDispatchers|CreateEvent :!event HandleTimerEvent) (Math|Timespan|GetTotalSeconds _outduration)))
    (Variables|Default|SetTimerHandle _returnvalue)
    (CallFunction|SetState "NewEnumerator1")
    (return true)
    (else
      (return false))))

(fn DeactivateAbility
  (if (Utilities|Enum|Equal(Enum) (Variables|Default|GetCurrentState) "NewEnumerator1")
    (bind _outcooldown (CallFunction|GetMaxCooldown))
    (bind _returnvalue (Utilities|Time|SetTimerbyEvent (EventDispatchers|CreateEvent :!event HandleTimerEvent) (Math|Timespan|GetTotalSeconds (+ _outcooldown (.OutTimspan (CallFunction|GetState))))))
    (Variables|Default|SetTimerHandle _returnvalue)
    (CallFunction|SetState "NewEnumerator2")
    (return true)
    (else
      (Development|PrintString "Can't deactivate a non-active ability")
      (return false))))

(fn GetState
  (bind _timerhandle (Variables|Default|GetTimerHandle))
  (bind _returnvalue (Utilities|Time|GetTimerRemainingTimebyHandle _timerhandle))
  (if (and (Utilities|Time|IsTimerActivebyHandle (Variables|Default|GetTimerHandle)) (Utilities|Enum|NotEqual(Enum) (Variables|Default|GetCurrentState) "NewEnumerator0"))
    (LocalVariables|SetReturnTimespan (Math|Timespan|MakeTimespan 0 0 0 (Math|Float|Truncate _returnvalue) (Math|Float|Truncate (* 1000 (Math|Float|Fraction _returnvalue)))))
    (else
      (LocalVariables|SetReturnTimespan (Math|Timespan|MakeTimespan 0))))
  (return (Variables|Default|GetCurrentState) (LocalVariables|GetReturnTimespan)))

(fn IsReady
  (return (Utilities|Enum|Equal(Enum) (Variables|Default|GetCurrentState) "NewEnumerator0")))

(fn IsActive
  (return (Utilities|Enum|Equal(Enum) (Variables|Default|GetCurrentState) "NewEnumerator1")))

(fn IsonCooldown
  (return (Utilities|Enum|Equal(Enum) (Variables|Default|GetCurrentState) "NewEnumerator2")))

(fn GetMaxDuration
  (bind _returnvalue (Utilities|GetDataTableRow (Variables|Default|GetDatatable) (Utilities|String|StringToName (CallFunction|GetAbilityString (Variables|Default|GetAbilityType) (Variables|Default|GetAbilityEnum))))
    (:then
      (LocalVariables|SetRetDuration (.Duration (Utilities|Struct|BreakAbilityDataEntry _returnvalue))))
    (:RowNotFound
      (Development|PrintString (Utilities|String|Append "Error Didn't find row for : " (CallFunction|GetAbilityString (Variables|Default|GetAbilityType) (Variables|Default|GetAbilityEnum)) ": In datatable : " (Utilities|GetDisplayName (Variables|Default|GetDatatable))))
      (LocalVariables|SetRetDuration (Math|Timespan|MakeTimespan 0))))
  (return (LocalVariables|GetRetDuration)))

(fn GetMaxCooldown
  (bind _returnvalue (Utilities|GetDataTableRow (Variables|Default|GetDatatable) (Utilities|String|StringToName (CallFunction|GetAbilityString (Variables|Default|GetAbilityType) (Variables|Default|GetAbilityEnum))))
    (:then
      (LocalVariables|SetRetCooldown (.Cooldown (Utilities|Struct|BreakAbilityDataEntry _returnvalue))))
    (:RowNotFound
      (LocalVariables|SetRetCooldown (Math|Timespan|MakeTimespan 0))))
  (return (LocalVariables|GetRetCooldown)))

(fn SetState
  (params (NewState :type EAbilityState%20Enum :default "NewEnumerator0"))
  (bind _output_get (Variables|Default|SetCurrentState NewState))
  (Default|CallAbilityStateChange (Variables|Default|GetAbilityType) (Variables|Default|GetAbilityEnum) _output_get))

(fn HandleTimerEvent
  (switch Utilities|FlowControl|Switch|SwitchonEAbilityState (Variables|Default|GetCurrentState)
    (:NewEnumerator0
      (Development|PrintString "We shouldn't have set a timer when in state Ready"))
    (:NewEnumerator1
      (CallFunction|SetState "NewEnumerator2")
      (bind _outcooldown (CallFunction|GetMaxCooldown))
      (bind _returnvalue (Utilities|Time|SetTimerbyEvent (EventDispatchers|CreateEvent :!event HandleTimerEvent) (Math|Timespan|GetTotalSeconds _outcooldown)))
      (Variables|Default|SetTimerHandle _returnvalue))
    (:NewEnumerator2
      (CallFunction|SetState "NewEnumerator0"))))